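; BP_WallSconce is a wall lamp with a cone-shaped light component, SconceLight, that can be switched on and off.
; The construction script sets the light's visibility from IsOn and applies the brightness, color and inner and outer cone angle variables.
; ToggleOn stores the requested state in IsOn and updates the light's visibility to match.
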(fn `ToggleOn`
  (params (TurnOn :type Boolean))
  (bind _output_get (set `self.IsOn` TurnOn)) ; Toto je už premenná ktorú máme, set znamená, že nastavujeme hodnotu, že svieti.
  (`SceneComponent.SetVisibility` (`self.SconceLight`) _output_get false) ; Je viditeľné keď
)

(fn `UserConstructionScript`
  (bind _sconcelight (`self.SconceLight`))
  (`|ExecutionSequence`
    (:`then_0`
      (`SceneComponent.SetVisibility` (`self.SconceLight`) (`self.IsOn`) false) ; Je viditeľné keď
    )
    (:`then_1`
      (`LightComponent.SetIntensity` _sconcelight (`self.Brightness`))
      (`LightComponent.SetLightColor` _sconcelight (`self.Color`) true)
      (`SpotLightComponent.SetInnerConeAngle` _sconcelight (`self.Inner Cone Angle`))
      (`SpotLightComponent.SetOuterConeAngle` _sconcelight (`self.Outer Cone Angle`)))))