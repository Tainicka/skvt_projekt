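; Player controller that lets the player swap between BP_SkvtBaseChar characters and toggle the main menu.
; On BeginPlay it adds the default and pawn-swap Enhanced Input mapping contexts.
; IA_Swap gathers all characters in the level and possesses the one after the current pawn, wrapping to the first at the end.
; IA_OpenMenu uses the stored widget reference's validity to open or close WBP_MainMenu, switching pause, cursor and input mode.
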(event `self.ReceiveBeginPlay`
  (bind _returnvalue (pcsubsystem `EnhancedInputLocalPlayerSubsystem` self))
  (`/Engine/EditorBlueprintResources/StandardMacros.IsValid` _returnvalue
    (:`Is Valid`
      (`EnhancedInputSubsystemInterface.AddMappingContext` _returnvalue "/Game/Skvt/Input/IMC_Default.IMC_Default" 0 (struct))
      (`EnhancedInputSubsystemInterface.AddMappingContext` _returnvalue "/Game/Skvt/Characters/Input/IMC_SwapPawn.IMC_SwapPawn" 0 (struct)) ; Pre swap musím pridať aj mapping context, v ktorom sa swap nachádza
    )))

(event `EnhancedInput|/Game/Skvt/Characters/Input/Actions/IA_Swap`
  (params (ActionValue :type Boolean) (ElapsedSeconds :type "Float (double-precision)") (TriggeredSeconds :type "Float (double-precision)") (InputAction :type "InputAction Object Reference" :default "/Game/Skvt/Characters/Input/Actions/IA_Swap.IA_Swap"))
  (:`Triggered`
    (bind _outactors (`GameplayStatics.GetAllActorsOfClass` "/Game/Skvt/Characters/BP_SkvtBaseChar.BP_SkvtBaseChar_C")) ; Nájdi všetky postavy a znich vyber jednu nasleduje
    (`self.Possess` (`self.FindNextCharacter` _outactors)) ; posadni jednu, čo si našiel
  ))

(event `EnhancedInput|/Game/Skvt/Input/Actions/IA_OpenMenu`
  (params (ActionValue :type Boolean) (ElapsedSeconds :type "Float (double-precision)") (TriggeredSeconds :type "Float (double-precision)") (InputAction :type "InputAction Object Reference" :default "/Game/Skvt/Input/Actions/IA_OpenMenu.IA_OpenMenu"))
  (:`Triggered`
    (`/Engine/EditorBlueprintResources/StandardMacros.IsValid` (`self.MainMenuRef`) ; je main menu otvorené - funguje ako branch ale funguje na objekty
      (:`Is Valid`
        (`self.CloseMenu`))
      (:`Is Not Valid`
        (`self.OpenMenu`)))))

(fn `CloseMenu`
  (`Widget.RemoveFromParent` (`self.MainMenuRef`))
  (set `self.MainMenuRef` null)
  (`WidgetBlueprintLibrary.SetInputMode_GameOnly` self)
  (set `self.bShowMouseCursor` false)
  (`GameplayStatics.SetGamePaused` false))

(fn `FindNextCharacter`
  (params (AllCharacters :type "Array of Pawn Object Reference"))
  (returns (NewCharacter :type "Pawn Object Reference"))
  (bind _returnvalue (`KismetArrayLibrary.Array_Find` AllCharacters (`self.K2_GetPawn`)))
  (bind _returnvalue_2 (+ _returnvalue 1))
  (if (>= _returnvalue 0)
    (if (== _returnvalue_2 (`KismetArrayLibrary.Array_Length` AllCharacters))
      (return (`|GetArrayItem` (`local.AllCharacters`))) ; toto mi vráti ćíslo, ak ju nájde, dostanem 1,2,3 ak ju nevráti, dostanem -1
      (else
        (return (`|GetArrayItem` (`local.AllCharacters`) _returnvalue_2)) ; toto mi vráti ćíslo, ak ju nájde, dostanem 1,2,3 ak ju nevráti, dostanem -1
      ))))

(fn `OpenMenu`
  (bind _returnvalue (`|CreateWidget` "/Game/Skvt/UI/Widgets/Menu/WBP_MainMenu.WBP_MainMenu_C" self))
  (bind _output_get (set `self.MainMenuRef` _returnvalue))
  (`UserWidget.AddToViewport` _output_get 0)
  (`WidgetBlueprintLibrary.SetInputMode_GameAndUIEx` self (`self.MainMenuRef`))
  (set `self.bShowMouseCursor` true)
  (`GameplayStatics.SetGamePaused` true))

(fn `UserConstructionScript`)